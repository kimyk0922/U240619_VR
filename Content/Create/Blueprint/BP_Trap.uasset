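; BP_Trap is a trap actor whose static mesh can be stepped along its local Y axis or hidden.
; MoveTo adds a fixed step to a running Value and applies it as the mesh's relative Y position only while below an upper limit.
; Visibility hides the mesh without propagating to children.
; The file shows no trigger for either function, and the construction script is empty.
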(fn `MoveTo`
  (bind _output_get (set `self.Value` (+ (`self.Value`) 400.0)))
  (if (< (`self.Value`) 2500.0)
    (`SceneComponent.K2_SetRelativeLocation` (`self.StaticMesh`) (`KismetMathLibrary.MakeVector` 0.0 _output_get) false false)))

(fn `UserConstructionScript`)

(fn `Visibility`
  (`SceneComponent.SetVisibility` (`self.StaticMesh`) false false))